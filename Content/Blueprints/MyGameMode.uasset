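; Game mode for a timed ambient listening session that plays layered bird, river and wind sounds.
; On BeginPlay it builds a Tracks array of structs pairing each cue with a 2D audio component, name and image, then fades all of them in.
; A timer set to PlayTime calls EndListening, which fades the sounds out, shows the end-of-listening widget and switches to mouse-driven UI-only input.
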(event EventBeginPlay
  (Utilities|Time|SetTimerbyFunctionName 0 "EndListening" (Variables|Default|GetPlayTime))
  (CallFunction|GenerateTrack)
  (CallFunction|PlayAllSound))

(fn ConstructionScript)

(fn EndListening
  (bind _returnvalue (Game|GetPlayerController 0))
  (CallFunction|StopAllSound)
  (bind _returnvalue_2 (UserInterface|CreateWidget "/Game/UI/W_EndOfListening.W_EndOfListening_C" _returnvalue))
  (UserInterface|Viewport|AddtoViewport _returnvalue_2 0)
  (Variables|/Script/Engine.PlayerController|SetbShowMouseCursor _returnvalue true)
  (Input|SetInputModeUIOnly _returnvalue _returnvalue_2 "DoNotLock"))

(fn StopAllSound
  (for _array_element (Variables|Default|GetTracks)
    (Audio|Components|Audio|FadeOut (.AudioComponent (Utilities|Struct|BreakTracks _array_element)) 1.0 0.0 :!class /Script/Engine.AudioComponent)))

(fn GenerateTrack
  (bind _returnvalue (Audio|CreateSound2D "/Game/Sound/Forest/Birds_Cue.Birds_Cue"))
  (Utilities|Array|Add (Variables|Default|GetTracks) (Utilities|Struct|MakeTracks "/Game/Sound/Forest/Birds_Cue.Birds_Cue" _returnvalue "Birds" "/Game/Art/Icons/Bird.Bird"))
  (bind _returnvalue_2 (Audio|CreateSound2D "/Game/Sound/Forest/River2_Cue.River2_Cue"))
  (Utilities|Array|Add (Variables|Default|GetTracks) (Utilities|Struct|MakeTracks "/Game/Sound/Forest/River2_Cue.River2_Cue" _returnvalue_2 "River" "/Game/Art/Icons/River.River"))
  (bind _returnvalue_3 (Audio|CreateSound2D "/Game/Sound/Forest/Wind_Cue.Wind_Cue"))
  (Utilities|Array|Add (Variables|Default|GetTracks) (Utilities|Struct|MakeTracks "/Game/Sound/Forest/Wind_Cue.Wind_Cue" _returnvalue_3 "Wind" "/Game/Art/Icons/Wind.Wind")))

(fn PlayAllSound
  (for _array_element (Variables|Default|GetTracks)
    (Audio|Components|Audio|FadeIn (.AudioComponent (Utilities|Struct|BreakTracks _array_element)) 5.0 1.0 0.0 :!class /Script/Engine.AudioComponent)))